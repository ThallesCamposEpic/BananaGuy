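; HUD that creates the main WB_Main widget and drives the start countdown, pause menu and game result screen.
; BeginPlay disables player input while a looping timer counts down, then shows "GO!!" and re-enables it.
; GameResult shows the given message, plays its animation, then reveals the end buttons with the cursor.
; OpenPauseMenu toggles the pause widget via FlipFlop, setting Game-and-UI input on both open and close.
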(event Custom|OpenPauseMenu
  (bind _main (Variables|Default|GetMain))
  (bind _wb_pausemenu (Variables|/Game/PrimeiroGame/Widgets/WB_Main.WB_Main_C|GetWB_PauseMenu _main))
  ;[1 1 1] Define a visibilidade de widget de menu
  (Utilities|FlowControl|FlipFlop
    (:A
      (Widget|SetVisibility _wb_pausemenu "Visible")
      ;[1 1 1] Define o tipo de input ao abri e fechar o menu
      (CallFunction|SetInputModeGameandUI))
    (:B
      (Widget|SetVisibility _wb_pausemenu "Collapsed")
      (CallFunction|SetInputModeGameandUI))))

(event Custom|GameResult
  (params (ResultMsg :type Text))
  ;[1 1 1] Adiciona a mensagem de vitória ou derrota dependendo da condição do jgo
  (Variables|/Game/PrimeiroGame/Widgets/WB_Main.WB_Main_C|SetGameResultMsg (Variables|Default|GetMain) ResultMsg)
  ;[1 1 1] Deixa o resultado do jogo visivel se der GameOver
  (Variables|/Script/UMG.Widget|SetVisibility (Variables|/Game/PrimeiroGame/Widgets/WB_Main.WB_Main_C|GetLifeBox (Variables|Default|GetMain)) "Visible")
  (Variables|/Script/UMG.Widget|SetVisibility (Variables|/Game/PrimeiroGame/Widgets/WB_Main.WB_Main_C|GetGameResultBox (Variables|Default|GetMain)) "Visible")
  ;[1 1 1] Inicia a animação de GameResult ao perder todas as vidas, após 5seg reseta o level
  (Components|Animation|PlayAnimation (Variables|Default|GetMain) (Variables|/Game/PrimeiroGame/Widgets/WB_Main.WB_Main_C|GetGameResultAnim (Variables|Default|GetMain)) 0.0
    (:Finished
      (Widget|SetVisibility (Variables|/Game/PrimeiroGame/Widgets/WB_Main.WB_Main_C|GetEndButtons (Variables|Default|GetMain)) "Visible")
      (CallFunction|SetInputModeGameandUI))))

(event Custom|CountDown
  (if (> (Variables|Default|GetCountDownValue) 0)
    (Rendering|Components|TextRender|SetText (Variables|/Game/PrimeiroGame/Widgets/WB_Main.WB_Main_C|GetCountDown (Variables|Default|GetMain)) (Utilities|Text|ToText(Integer) (Variables|Default|GetCountDownValue)))
    (Math|Integer|DecrementInt (Variables|Default|GetCountDownValue))
    (else
      (Utilities|Time|ClearandInvalidateTimerbyHandle (Variables|Default|GetTimerHandler))
      (Rendering|Components|TextRender|SetText (Variables|/Game/PrimeiroGame/Widgets/WB_Main.WB_Main_C|GetCountDown (Variables|Default|GetMain)) "GO!!")
      (Input|EnableInput (Game|GetPlayerCharacter 0) (Game|GetPlayerController 0))
      (Utilities|FlowControl|Delay 2.0)
      (Widget|SetVisibility (Variables|/Game/PrimeiroGame/Widgets/WB_Main.WB_Main_C|GetCountDown (Variables|Default|GetMain)) "Collapsed"))))

(event EventBeginPlay
  (CallFunction|SetInputModeGameOnly)
  ;[1 1 1] Cria o widget com base na classe informada
  (bind _returnvalue (UserInterface|CreateWidget "/Game/PrimeiroGame/Widgets/WB_Main.WB_Main_C" (Game|Player|GetOwningPlayerController)))
  ;[1 1 1] Salva a referencia do widget criado
  (bind _output_get (Variables|Default|SetMain _returnvalue))
  ;[1 1 1] Adiciona o Widget em tela
  (UserInterface|Viewport|AddtoViewport _output_get 0)
  (Variables|/Script/UMG.Widget|SetVisibility (Variables|/Game/PrimeiroGame/Widgets/WB_Main.WB_Main_C|GetCountDown (Variables|Default|GetMain)) "Visible")
  (bind _returnvalue_2 (Utilities|Time|SetTimerbyEvent (delegate Custom|CountDown) 1.0 true))
  (Variables|Default|SetTimerHandler _returnvalue_2)
  (Input|DisableInput (Game|GetPlayerCharacter 0) (Game|GetPlayerController 0)))

(fn ConstructionScript)

(fn SetInputModeGameandUI
  (Input|SetInputModeGameandUI (Game|GetPlayerController 0) 0 "DoNotLock" true false)
  (Variables|/Script/Engine.PlayerController|SetbShowMouseCursor (Game|GetPlayerController 0) true))

(fn SetInputModeGameOnly
  (Input|SetInputModeGameOnly (Game|GetPlayerController 0) false)
  (Variables|/Script/Engine.PlayerController|SetbShowMouseCursor (Game|GetPlayerController 0) false))
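; BP_Player_Banana is a player Character with movement, camera look and jump driven by Enhanced Input actions.
; Movement follows the control rotation's yaw, while camera input feeds controller yaw and pitch.
; An ActiveRagdoll event calls the Ragdoll function, which switches the mesh to ragdoll collision with simulated physics and disables movement, then destroys the actor after a short delay.
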(event Custom|ActiveRagdoll
  ;[1 1 1] Ativa o Ragdoll, espera 2seg e destrói a classe
  (CallFunction|Ragdoll)
  (Utilities|FlowControl|Delay 2.0)
  (Actor|DestroyActor))

(event Input|EnhancedActionEvents|EnhancedInputActionIA_Camera
  (params (ActionValue :type Vector%202D%20Structure) (ElapsedSeconds :type Float%20%28double-precision%29) (TriggeredSeconds :type Float%20%28double-precision%29) (InputAction :type Input%20Action%20Object%20Reference :default "/Game/PrimeiroGame/Player/Inputs/IA_Camera.IA_Camera"))
  ;[1 1 1] Evento de movimentação da câmera
  (Pawn|Input|AddControllerYawInput (.x ActionValue))
  (Pawn|Input|AddControllerPitchInput (.y ActionValue)))

(event Input|EnhancedActionEvents|EnhancedInputActionIA_Moviment
  (params (ActionValue :type Vector%202D%20Structure) (ElapsedSeconds :type Float%20%28double-precision%29) (TriggeredSeconds :type Float%20%28double-precision%29) (InputAction :type Input%20Action%20Object%20Reference :default "/Game/PrimeiroGame/Player/Inputs/IA_Moviment.IA_Moviment"))
  ;[1 1 1] Evento de movimentação do personagem WASD
  ;;[1 1 1] Add movimento na Dir/Esq
  (Pawn|Input|AddMovementInput (Math|Vector|GetRightVector (Math|Rotator|MakeRotator 0.0 0.0 (.yaw (Pawn|GetControlRotation :!class /Script/Engine.Pawn)))) (.x ActionValue) false)
  ;;[1 1 1] Add movimento Frente/Trás
  (Pawn|Input|AddMovementInput (Math|Vector|GetForwardVector (Math|Rotator|MakeRotator 0.0 0.0 (.yaw (Pawn|GetControlRotation :!class /Script/Engine.Pawn)))) (.y ActionValue) false))

(event Input|EnhancedActionEvents|EnhancedInputActionIA_Jump
  (params (ActionValue :type Boolean) (ElapsedSeconds :type Float%20%28double-precision%29) (TriggeredSeconds :type Float%20%28double-precision%29) (InputAction :type Input%20Action%20Object%20Reference :default "/Game/PrimeiroGame/Player/Inputs/IA_Jump.IA_Jump"))
  ;[1 1 1] Evento de pulo do jogador
  (:Started
    (Character|Jump))
  (:Canceled
    (Character|StopJumping)))

(fn ConstructionScript)

(fn Ragdoll
  ;[1 1 1] Função para o Ragdoll
  ;;[1 1 1] Função Ragdoll
  ;;[1 1 1] Define um novo preset de colisão
  (Collision|SetCollisionProfileName (Variables|Character|GetMesh) "Ragdoll" true :!class /Script/Engine.PrimitiveComponent)
  ;;[1 1 1] Ativa o simular fisica
  (Physics|SetSimulatePhysics (Variables|Character|GetMesh) true)
  ;;[1 1 1] Desabilita o movimento
  (Pawn|Components|CharacterMovement|DisableMovement (Variables|Character|GetCharacterMovement)))
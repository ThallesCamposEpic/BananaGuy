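; BP_SpinningPlate is a trap actor with a plate that spins around its yaw axis.
; On BeginPlay it feeds RotationSpeed into the RotatingMovement component's rotation rate, so the sign sets the spin direction.
; For negative speeds it also rolls each direct child of Plate by 180 degrees, flipping the attached parts to match the reversed spin.
; No Tick or overlap logic runs.
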(event EventBeginPlay
  ;[1 1 1] Executa uma unica vez ao iniciar o jogo
  ;;[1 1 1] Define o valor de velocidade do prato
  (Variables|/Script/Engine.RotatingMovementComponent|SetRotationRate (Variables|Default|GetRotatingMovement) (Math|Rotator|MakeRotator 0.0 0.0 (Variables|Default|GetRotationSpeed)))
  ;;[1 1 1] Valida se a velocidade do prato é negativa
  (if (< (Variables|Default|GetRotationSpeed) 0.0)
    ;;[1 1 1] Para cada filho pegamos o valor atual de rotação e add 180 graus ao eixo Roll(x)
    (for _array_element (Components|GetChildrenComponents (Variables|Default|GetPlate) false)
      (Transformation|SetRelativeRotation _array_element (Math|Rotator|MakeRotator (+ (.roll (Variables|/Script/Engine.SceneComponent|GetRelativeRotation _array_element)) 1.8e+02) (.pitch (Variables|/Script/Engine.SceneComponent|GetRelativeRotation _array_element)) (.yaw (Variables|/Script/Engine.SceneComponent|GetRelativeRotation _array_element))) false false))))

(event Collision|EventActorBeginOverlap
  (params (OtherActor :type Actor%20Object%20Reference)))

(event EventTick
  (params (DeltaSeconds :type Float%20%28single-precision%29)))

(fn ConstructionScript)